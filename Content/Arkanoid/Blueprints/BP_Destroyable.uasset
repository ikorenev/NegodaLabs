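; Destroyable Arkanoid brick that takes hits from the game ball and awards points when destroyed.
; On spawn it rolls a random health of one to three and creates a dynamic material on its cube.
; Each ball hit lowers health, recoloring the cube through a health-indexed color parameter or destroying the actor at zero.
; The Destroyed event tells BP_GameMode to add points.
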(event `self.ReceiveBeginPlay`
  (set `self.Health` (`KismetMathLibrary.RandomIntegerInRange` 1 3))
  (bind _returnvalue (`KismetMaterialLibrary.CreateDynamicMaterialInstance` "/Game/Arkanoid/Blueprints/M_Color.M_Color"))
  (bind _output_get (set `self.CubeMaterial` _returnvalue))
  (`PrimitiveComponent.SetMaterial` (`self.Cube`) 0 _output_get)
  (`self.SetColorByHealth`))

(event `self.ReceiveHit`
  (params (MyComp :type "PrimitiveComponent Object Reference") (Other :type "Actor Object Reference") (OtherComp :type "PrimitiveComponent Object Reference") (bSelfMoved :type Boolean) (HitLocation :type "Vector Structure") (HitNormal :type "Vector Structure") (NormalImpulse :type "Vector Structure") (Hit :type "HitResult Structure (by ref)"))
  (bind _health (`self.Health`))
  (cast `/Game/Arkanoid/Blueprints/BP_GameBall` Other)
  (`/Engine/EditorBlueprintResources/StandardMacros.DecrementInt` _health
    (:`  `
      (`/Engine/EditorBlueprintResources/StandardMacros.CompareInt` _health
        (:`>`
          (`self.SetColorByHealth`))
        (:`==`
          (`self.K2_DestroyActor`))))))

(event `self.ReceiveDestroyed`
  (bind _asbp_game_mode (cast `/Game/Arkanoid/Blueprints/BP_GameMode` (`GameplayStatics.GetGameMode`)))
  (`/Game/Arkanoid/Blueprints/BP_GameMode.AddPoints` _asbp_game_mode))

(fn `SetColorByHealth`
  (`MaterialInstanceDynamic.SetVectorParameterValue` (`self.CubeMaterial`) "Color" (select `int` (`self.Health`) :`0` (struct) :`1` (struct :`R` 1.0 :`B` 0.053367 :`A` 1.0) :`2` (struct :`R` 1.0 :`G` 0.967587 :`A` 1.0) :`3` (struct :`G` 1.0 :`B` 0.03602 :`A` 1.0) :!type "LinearColor Structure")))

(fn `UserConstructionScript`)