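; Game mode for an Arkanoid game that tracks points and lives and drives ball spawning and game over.
; BeginPlay shows the GUI widget, then loops through a short Delay, repeatedly calling SpawnTheBall on the player's BP_Pawn.
; AddPoints raises the score by a fixed amount.
; ReduceLives decrements lives, then either pauses and shows the game-over widget at zero or asks the pawn for another ball.
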(event `self.ReceiveBeginPlay`
  (bind _returnvalue (`|CreateWidget` "/Game/Arkanoid/Blueprints/BP_GUI.BP_GUI_C"))
  (bind _output_get (set `self.Widget` _returnvalue))
  (`UserWidget.AddToViewport` _output_get 0)
  (bind _asbp_pawn (cast `/Game/Arkanoid/Blueprints/BP_Pawn` (`GameplayStatics.GetPlayerPawn` 0)))
  (`/Game/Arkanoid/Blueprints/BP_Pawn.SpawnTheBall` _asbp_pawn :!label _label)
  (`KismetSystemLibrary.Delay` 0.2)
  (goto _label))

(event `AddPoints`
  (set `self.Points` (+ (`self.Points`) 100)))

(event `ReduceLives`
  (bind _result (`/Engine/EditorBlueprintResources/StandardMacros.DecrementInt` (`self.Lives`))
    (:`  `
      (if (== _result 0)
        (`GameplayStatics.SetGamePaused` true)
        (bind _returnvalue (`|CreateWidget` "/Game/Arkanoid/Blueprints/BP_GameOver.BP_GameOver_C"))
        (`UserWidget.AddToViewport` _returnvalue 0)
        (else
          (bind _asbp_pawn (cast `/Game/Arkanoid/Blueprints/BP_Pawn` (`GameplayStatics.GetPlayerPawn` 0)))
          (`/Game/Arkanoid/Blueprints/BP_Pawn.SpawnTheBall` _asbp_pawn))))))

(fn `UserConstructionScript`)