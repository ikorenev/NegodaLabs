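; BP_GameBall is the Arkanoid ball, which moves itself and bounces off whatever it hits.
; Each Tick sweeps it along Direction at BallSpeed, reflecting off blocking hits and normalizing in XY.
; Hits on BP_Pawn first nudge Direction by a constant delta signed by the pawn's Y movement direction.
; Overlapping a KillZVolume destroys the ball, and its Destroyed event calls ReduceLives on BP_GameMode.
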(event `self.ReceiveActorBeginOverlap`
  (params (OtherActor :type "Actor Object Reference"))
  (cast `KillZVolume` OtherActor)
  (`self.K2_DestroyActor`))

(event `self.ReceiveTick`
  (params (DeltaSeconds :type "Float (single-precision)"))
  (bind _constantdirectiondelta (`self.ConstantDirectionDelta`))
  (bind _direction (`self.Direction`))
  (bind _sweephitresult (`self.K2_AddActorWorldOffset` (* (* (`self.Direction`) (`self.BallSpeed`)) DeltaSeconds) true))
  (bind (_bblockinghit _binitialoverlap _time _distance _location _impactpoint _normal _impactnormal _physmat _hitactor) (`GameplayStatics.BreakHitResult` _sweephitresult))
  (if _bblockinghit
    (bind _asbp_pawn (cast `/Game/Arkanoid/Blueprints/BP_Pawn` _hitactor)
      (:`then`
        (bind (_currentdirection_x _currentdirection_y) (`KismetMathLibrary.BreakVector` (`/Game/Arkanoid/Blueprints/BP_Pawn.CurrentDirection` _asbp_pawn)))
        ;[1 1 1] Constant direction change
        (`/Engine/EditorBlueprintResources/StandardMacros.CompareFloat` _currentdirection_y
          (:`>`
            (set `self.Direction` (+ _direction _constantdirectiondelta)))
          (:`==`
            _)
          (:`<`
            (set `self.Direction` (+ _direction (* _constantdirectiondelta -1.0))))))
      (:`CastFailed`
        _))
    (bind (_returnvalue_x _returnvalue_y) (`KismetMathLibrary.BreakVector` (`KismetMathLibrary.GetReflectionVector` (`self.Direction`) _normal)))
    ;[1 1 1] Reflection Calculation
    (set `self.Direction` (`KismetMathLibrary.Normal` (`KismetMathLibrary.MakeVector` _returnvalue_x _returnvalue_y)))))

(event `self.ReceiveDestroyed`
  (bind _asbp_game_mode (cast `/Game/Arkanoid/Blueprints/BP_GameMode` (`GameplayStatics.GetGameMode`)))
  (`/Game/Arkanoid/Blueprints/BP_GameMode.ReduceLives` _asbp_game_mode))

(fn `UserConstructionScript`)