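; BP_FloorGenerator builds a grid floor from a user-supplied static mesh, sized by horizontal and vertical tile counts.
; Its Construction Script runs nested loops that add a separate Static Mesh Component per cell at a fixed 300-unit spacing, with rows starting one cell out along Y.
; The Event Graph holds only disabled default events, so it adds no runtime logic.
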(fn `UserConstructionScript`
  (for _index (range (`self.CountVertical`))
    (for _index_2 (range (`self.CountHorizontal`))
      (bind _returnvalue (`AddComponent|NODE_AddStaticMeshComponent-0` :`RelativeTransform` (`KismetMathLibrary.MakeTransform` (`KismetMathLibrary.MakeVector` (`KismetMathLibrary.Conv_IntToDouble` (* _index_2 300)) (`KismetMathLibrary.Conv_IntToDouble` (+ (* _index 300) 300))))))
      (`StaticMeshComponent.SetStaticMesh` _returnvalue (`self.UserMesh`)))))