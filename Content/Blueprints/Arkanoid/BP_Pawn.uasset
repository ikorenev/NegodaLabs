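; BP_Pawn is the player-controlled pawn for an Arkanoid game, moving sideways as the paddle.
; The PlatformMove axis drives a swept local Y offset scaled by Speed and world delta time.
; SpawnTheBall creates a scaled-down BP_GameBall at BallSpawnPlace's transform, but is not called within this Blueprint.
; Key 1 runs a FlipFlop whose branches both show the mouse cursor, so it never hides it.
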(event `InputAxis|PlatformMove`
  (params (AxisValue :type "Float (single-precision)"))
  (bind _output_get (set `self.CurrentDirection` (`KismetMathLibrary.MakeVector` 0.0 (* (`self.Speed`) (`GameplayStatics.GetWorldDeltaSeconds`) AxisValue))))
  (`self.K2_AddActorLocalOffset` _output_get true))

(event `Key|One`
  (params (Key :type "Key Structure"))
  (bind _returnvalue (`GameplayStatics.GetPlayerController` 0))
  (:`Pressed`
    (`/Engine/EditorBlueprintResources/StandardMacros.FlipFlop`
      (:`A`
        (set `PlayerController.bShowMouseCursor` true _returnvalue))
      (:`B`
        (set `PlayerController.bShowMouseCursor` true _returnvalue)))))

(fn `SpawnTheBall`
  (bind (_returnvalue_location _returnvalue_rotation) (`KismetMathLibrary.BreakTransform` (`SceneComponent.K2_GetComponentToWorld` (`self.BallSpawnPlace`))))
  (`|SpawnActorFromClass` "/Game/Blueprints/Arkanoid/BP_GameBall.BP_GameBall_C" (`KismetMathLibrary.MakeTransform` _returnvalue_location _returnvalue_rotation (0.1 0.1 0.1)) "Undefined" "OverrideRootScale" null null))

(fn `UserConstructionScript`)