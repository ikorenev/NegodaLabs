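; BP_Generator is the Arkanoid level generator that builds a grid of BP_Destroyable blocks.
; Its Construction Script loops over Rows and Columns, adding a scaled-down child actor component per cell at fixed X and Y spacing, offset one step from the origin.
; BeginPlay gathers all BP_Destroyable actors but does nothing with the result.
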(event `self.ReceiveBeginPlay`
  (`GameplayStatics.GetAllActorsOfClass` "/Game/Blueprints/Arkanoid/BP_Destroyable.BP_Destroyable_C"))

(fn `UserConstructionScript`
  (for _index (range 1 (+ (`self.Rows`) 1))
    (for _index_2 (range 1 (+ (`self.Columns`) 1))
      (bind _returnvalue (`AddComponent|NODE_AddChildActorComponent-0` :`RelativeTransform` (`KismetMathLibrary.MakeTransform` (+ (* (0.0 25.0 0.0) _index_2) (* (25.0 0.0 0.0) _index)) (struct) (0.125 0.125 0.125))))
      (`ChildActorComponent.SetChildActorClass` _returnvalue "/Game/Blueprints/Arkanoid/BP_Destroyable.BP_Destroyable_C"))))