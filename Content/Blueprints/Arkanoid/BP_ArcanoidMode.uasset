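; Trigger-box controller for an Arkanoid mini-game entered from third-person play, tracking score and lives.
; On overlap it blends to the arcade camera, hides the character, possesses BP_Pawn, then creates the GUI and spawns a ball.
; Losing a life respawns the ball, or pauses and shows BP_GameOver at zero.
; ExitGame removes the GUI, returns view and control to the character, and calls BP_Generator's Generate.
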(event `self.Box.OnComponentBeginOverlap`
  (params (OverlappedComponent :type "PrimitiveComponent Object Reference") (OtherActor :type "Actor Object Reference") (OtherComp :type "PrimitiveComponent Object Reference") (OtherBodyIndex :type Integer) (bFromSweep :type Boolean) (SweepResult :type "HitResult Structure (by ref)"))
  (cast `/Game/Blueprints/ThirdPerson/Blueprints/BP_ThirdPersonCharacter` OtherActor)
  (`self.ChangViewToGame`)
  (`KismetSystemLibrary.Delay` 0.5)
  (bind _returnvalue (`GameplayStatics.GetActorOfClass` "/Game/Blueprints/Arkanoid/BP_Pawn.BP_Pawn_C"))
  (`Controller.Possess` (`GameplayStatics.GetPlayerController` 0) _returnvalue)
  (bind _returnvalue_2 (`GameplayStatics.GetActorOfClass` "/Game/Blueprints/Arkanoid/BP_ArcanoidCamera.BP_ArcanoidCamera_C"))
  (`PlayerController.SetViewTargetWithBlend` (`GameplayStatics.GetPlayerController` 0) _returnvalue_2 0.0 "VTBlend_Linear" 0.0 false)
  (`self.InitGame`))

(event `ExitGame`
  (bind _returnvalue (`GameplayStatics.GetPlayerController` 0))
  (`Widget.RemoveFromParent` (`self.Widget`))
  (bind _returnvalue_2 (`GameplayStatics.GetActorOfClass` "/Game/Blueprints/ThirdPerson/Blueprints/BP_ThirdPersonCharacter.BP_ThirdPersonCharacter_C"))
  (`self.SetActorHiddenInGame` _returnvalue_2 false)
  (`PlayerController.SetViewTargetWithBlend` _returnvalue _returnvalue_2 0.5 "VTBlend_Linear" 0.0 false)
  (`KismetSystemLibrary.Delay` 0.5)
  (`Controller.Possess` _returnvalue _returnvalue_2)
  (`self.EnableInput` (`GameplayStatics.GetPlayerPawn` 0) (`GameplayStatics.GetPlayerController` 0))
  (bind _returnvalue_3 (`GameplayStatics.GetActorOfClass` "/Game/Blueprints/Arkanoid/BP_Generator.BP_Generator_C"))
  (`/Game/Blueprints/Arkanoid/BP_Generator.Generate` _returnvalue_3))

(event `AddPoints`
  (set `self.Points` (+ (`self.Points`) 100)))

(event `ReduceLives`
  (bind _result (`/Engine/EditorBlueprintResources/StandardMacros.DecrementInt` (`self.Lives`))
    (:`  `
      (if (== _result 0)
        (`GameplayStatics.SetGamePaused` true)
        (bind _returnvalue (`|CreateWidget` "/Game/Blueprints/Arkanoid/BP_GameOver.BP_GameOver_C"))
        (`UserWidget.AddToViewport` _returnvalue 0)
        (else
          (bind _asbp_pawn (cast `/Game/Blueprints/Arkanoid/BP_Pawn` (`GameplayStatics.GetPlayerPawn` 0)))
          (`/Game/Blueprints/Arkanoid/BP_Pawn.SpawnTheBall` _asbp_pawn))))))

(fn `ChangViewToGame`
  (bind _returnvalue (`GameplayStatics.GetPlayerController` 0))
  (bind _returnvalue_2 (`GameplayStatics.GetActorOfClass` "/Game/Blueprints/Arkanoid/BP_ArcanoidCamera.BP_ArcanoidCamera_C"))
  (`PlayerController.SetViewTargetWithBlend` _returnvalue _returnvalue_2 0.5 "VTBlend_Linear" 0.0 false)
  (`self.SetActorHiddenInGame` (`GameplayStatics.GetPlayerPawn` 0) true)
  (`self.DisableInput` _returnvalue _returnvalue)
  (`self.DisableInput` (`GameplayStatics.GetPlayerPawn` 0) _returnvalue))

(fn `InitGame`
  (bind _returnvalue (`|CreateWidget` "/Game/Blueprints/Arkanoid/BP_GUI.BP_GUI_C"))
  (bind _output_get (set `self.Widget` _returnvalue))
  (`UserWidget.AddToViewport` _output_get 0)
  (bind _asbp_pawn (cast `/Game/Blueprints/Arkanoid/BP_Pawn` (`GameplayStatics.GetPlayerPawn` 0)))
  (`/Game/Blueprints/Arkanoid/BP_Pawn.SpawnTheBall` _asbp_pawn)
  (set `self.Lives` (`self.MaxLives`))
  (set `self.Points` 0))

(fn `UserConstructionScript`)