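; Construction-script wall generator that builds a horizontal row of modular wall pieces as static mesh components.
; Each piece sits at a fixed spacing along local X and takes a random mesh from the UserMeshes array, re-rolled on every construction run.
; Optional inclined wood pillars appear at a set interval, either at the piece origin or shifted one segment along.
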(fn `UserConstructionScript`
  (bind _usermeshes (`self.UserMeshes`))
  (for _index (range (`self.CountHorizontal`))
    (bind _returnvalue (`KismetMathLibrary.Conv_IntToDouble` (* _index 300)))
    (bind _returnvalue_2 (`AddComponent|NODE_AddStaticMeshComponent-0` :`RelativeTransform` (`KismetMathLibrary.MakeTransform` (`KismetMathLibrary.MakeVector` _returnvalue))))
    (`StaticMeshComponent.SetStaticMesh` _returnvalue_2 (`|GetArrayItem` _usermeshes (`KismetMathLibrary.RandomIntegerInRange` 0 (- (`KismetArrayLibrary.Array_Length` _usermeshes) 1))))
    (if (`self.Pilars?`)
      (if (== (mod _index (`self.EveryWhallPilars`)) 0)
        (if (`self.Offset?`)
          (bind _returnvalue_3 (`AddComponent|NODE_AddStaticMeshComponent-2` :`RelativeTransform` (`KismetMathLibrary.MakeTransform` (`KismetMathLibrary.MakeVector` (+ _returnvalue 300.0)))))
          (`StaticMeshComponent.SetStaticMesh` _returnvalue_3 "/Game/Assets/Medieval_Environment/Medieval_Houses_Vol2/Meshes/SM_MH_02_Wood_Pillar_01_Inclined_01.SM_MH_02_Wood_Pillar_01_Inclined_01")
          (else
            (bind _returnvalue_4 (`AddComponent|NODE_AddStaticMeshComponent-1` :`RelativeTransform` (`KismetMathLibrary.MakeTransform` (`KismetMathLibrary.MakeVector` _returnvalue))))
            (`StaticMeshComponent.SetStaticMesh` _returnvalue_4 "/Game/Assets/Medieval_Environment/Medieval_Houses_Vol2/Meshes/SM_MH_02_Wood_Pillar_01_Inclined_01.SM_MH_02_Wood_Pillar_01_Inclined_01")))))))