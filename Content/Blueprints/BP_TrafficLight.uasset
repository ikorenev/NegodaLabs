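; Traffic light actor that cycles endlessly from red to yellow to green and straight back to red after BeginPlay.
; Two dynamic material instances, one lit and one black, are swapped between the three lamp meshes.
; The ChangeColor timeline animates the lit material's intensity before each switch.
; The ChangeMode macro then recolors it, holds red and green longer than yellow, and restarts the timeline.
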(event `self.ReceiveBeginPlay`
  (`self.SetDynamicMaterials`)
  (`KismetSystemLibrary.Delay` 2.0)
  (`self.ChangeMod`))

(event `ChangeMod`
  (bind (_direction _newtrack_0) (`Timeline|ChangeColor` :!via `PlayFromStart`)
    (:`Update`
      (`MaterialInstanceDynamic.SetScalarParameterValue` (`self.CurrentColor`) "LightIntensity" (`KismetMathLibrary.Lerp` 0.0 3.0 _newtrack_0)))
    (:`Finished`
      (switch `/Game/Blueprints/E_Color` (`self.NextColor`)
        (:`NewEnumerator0`
          (`self.ChangeMode` "NewEnumerator0" 8.0))
        (:`NewEnumerator1`
          (`self.ChangeMode` "NewEnumerator1" 0.1))
        (:`NewEnumerator2`
          (`self.ChangeMode` "NewEnumerator2" 8.0))))))

(fn `SetColor`
  (params (Color :type "/Game/Blueprints/E_Color Enum" :default "NewEnumerator0") (Material :type "MaterialInstanceDynamic Object Reference"))
  (switch `/Game/Blueprints/E_Color` Color
    (:`NewEnumerator0`
      (`MaterialInstanceDynamic.SetVectorParameterValue` Material "LightColor" (struct :`R` 1.0 :`B` 0.030088 :`A` 1.0)))
    (:`NewEnumerator1`
      (`MaterialInstanceDynamic.SetVectorParameterValue` Material "LightColor" (struct :`R` 0.978103 :`G` 1.0 :`A` 1.0)))
    (:`NewEnumerator2`
      (`MaterialInstanceDynamic.SetVectorParameterValue` Material "LightColor" (struct :`G` 1.0 :`B` 0.016937 :`A` 1.0)))
    (:`NewEnumerator3`
      (`MaterialInstanceDynamic.SetVectorParameterValue` :`self` Material :`ParameterName` "LightColor"))))

(fn `SetDynamicMaterials`
  (bind _inactivecolor (`self.InActiveColor`))
  (`|ExecutionSequence`
    (:`then_0`
      (bind _returnvalue (`PrimitiveComponent.CreateDynamicMaterialInstance` (`self.YelowColor`) 0 "/Game/Models/Materials/M_ColorForTraffic.M_ColorForTraffic" "None"))
      (set `self.InActiveColor` _returnvalue)
      (`PrimitiveComponent.SetMaterial` (`self.GreenColor`) 0 _inactivecolor)
      (`self.SetColor` "NewEnumerator3" _inactivecolor))
    (:`then_1`
      (bind _returnvalue_2 (`PrimitiveComponent.CreateDynamicMaterialInstance` (`self.RedColor`) 0 "/Game/Models/Materials/M_ColorForTraffic.M_ColorForTraffic" "None"))
      (bind _output_get (set `self.CurrentColor` _returnvalue_2))
      (`self.SetColor` "NewEnumerator0" _output_get)
      (set `self.NextColor` "NewEnumerator1"))))

(fn `UserConstructionScript`)