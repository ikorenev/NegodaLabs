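; BP_RoofGenerator is a construction-time generator that builds a horizontal row of randomly chosen meshes, presumably roof pieces.
; The construction script loops CountHorizontal times, picking a random entry from the UserMeshes array for each slot.
; An AddMesh function spawns a static mesh component at a fixed X spacing and assigns the mesh.
; Picks are unseeded, so the layout can change whenever construction reruns.
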(fn `Add Mesh`
  (params (NewMesh :type "StaticMesh Object Reference") (RelativeTransform_Location_X :type "Float (double-precision)"))
  (bind _returnvalue (`AddComponent|NODE_AddStaticMeshComponent-0` :`RelativeTransform` (`KismetMathLibrary.MakeTransform` (`KismetMathLibrary.MakeVector` RelativeTransform_Location_X))))
  (`StaticMeshComponent.SetStaticMesh` _returnvalue NewMesh))

(fn `UserConstructionScript`
  (bind _usermeshes (`self.UserMeshes`))
  (for _index (range (`self.CountHorizontal`))
    (`self.Add Mesh` (`|GetArrayItem` _usermeshes (`KismetMathLibrary.RandomIntegerInRange` 0 (- (`KismetArrayLibrary.Array_Length` _usermeshes) 1))) (`KismetMathLibrary.Conv_IntToDouble` (* _index 150)))))